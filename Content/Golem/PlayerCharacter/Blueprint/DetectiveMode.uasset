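; Player character Blueprint for a modular golem, with body parts following the main mesh via master pose.
; Input drives movement, consecutive jumps with growing hold time, montage punches toggling hand collision spheres, and an aim state when punching is off.
; A Copy dash grants brief invulnerability and opens the window for Transform to apply a fire helmet.
; Capsule hits gate damage, followed by timed immunity, and "HeadRemover" overlaps blow off the head, which regrows after a delay.
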(event OnComponentHit(CapsuleComponent)
  (params (HitComponent :type Primitive%20Component%20Object%20Reference) (OtherActor :type Actor%20Object%20Reference) (OtherComp :type Primitive%20Component%20Object%20Reference) (NormalImpulse :type Vector :default "0, 0, 0") (Hit :type Hit%20Result%20Structure%20%28by%20ref%29))
  ;[1 1 1] Character taking hits
  (Variables|Default|SetIs%20injured true)
  (Utilities|FlowControl|Delay 3.0)
  (Variables|Default|SetIs%20injured false))

(event OnComponentBeginOverlap(HeadSplitter)
  (params (OverlappedComponent :type Primitive%20Component%20Object%20Reference) (OtherActor :type Actor%20Object%20Reference) (OtherComp :type Primitive%20Component%20Object%20Reference) (OtherBodyIndex :type Integer) (bFromSweep :type Boolean) (SweepResult :type Hit%20Result%20Structure%20%28by%20ref%29))
  ;[1 1 1] Decapitation Feature
  (if (Actor|ActorHasTag OtherActor "HeadRemover")
    (Utilities|FlowControl|DoOnce false :!label _label
      (:Completed
        (Variables|Default|SetRegrowLimb 1)
        (Utilities|FlowControl|Sequence
          (:then_0
            (Utilities|FlowControl|Delay 5.0)
            (Variables|Default|SetRegrowLimb 0)
            (CallFunction|RegrowLeftArm)
            (goto _label Reset))
          (:then_1
            (switch int (Variables|Default|GetRegrowLimb)
              (:0
                (Class|SkinnedMeshComponent|SetSkeletalMesh (Variables|Default|GetHead) "/Game/Golem/PlayerCharacter/Blueprint/GolumParts/Head.Head" true)
                (Class|SkinnedMeshComponent|SetSkeletalMesh (Variables|Default|GetHelmet) "/Game/Golem/PlayerCharacter/Blueprint/GolumParts/Helmet.Helmet" true))
              (:1
                (Class|SkinnedMeshComponent|SetSkeletalMesh (Variables|Default|GetHead) 0 true)
                (Effects|SpawnEmitteratLocation "/Game/StarterContent/Particles/P_Explosion.P_Explosion" (Transformation|GetSocketLocation (Variables|Default|GetHeadSplitter) "Head"))))))))))

(event Custom|Damage%20Imunity%20time
  (Variables|Actor|SetbCanBeDamaged false)
  (Utilities|FlowControl|Delay 3.0)
  (Variables|Actor|SetbCanBeDamaged true))

(event Custom|Physical%20Animation%20activation
  ;[1 1 1] Physics (postponed)
)

(event Custom|RegrowLeftArm
  ;[1 1 1] Decapitation Feature
  (switch int (Variables|Default|GetRegrowLimb)
    (:0
      (Class|SkinnedMeshComponent|SetSkeletalMesh (Variables|Default|GetHead) "/Game/Golem/PlayerCharacter/Blueprint/GolumParts/Head.Head" true)
      (Class|SkinnedMeshComponent|SetSkeletalMesh (Variables|Default|GetHelmet) "/Game/Golem/PlayerCharacter/Blueprint/GolumParts/Helmet.Helmet" true))
    (:1
      (Class|SkinnedMeshComponent|SetSkeletalMesh (Variables|Default|GetHead) 0 true)
      (Effects|SpawnEmitteratLocation "/Game/StarterContent/Particles/P_Explosion.P_Explosion" (Transformation|GetSocketLocation (Variables|Default|GetHeadSplitter) "Head")))))

(event Custom|Transform
  (if (Variables|Default|GetIs%20copying)
    (Utilities|FlowControl|DoOnce false :!label _label
      (:Completed
        (Utilities|FlowControl|Sequence
          (:then_0
            (if (Variables|Default|GetHas%20Fire)
              (Development|PrintString "fire")
              (Class|SkinnedMeshComponent|SetSkeletalMesh (Variables|Default|GetHead) "/Game/Golem/PlayerCharacter/Blueprint/GolumParts/Transformations/Fire/Fire_Helmet.Fire_Helmet" true)
              (Class|SkinnedMeshComponent|SetSkeletalMesh (Variables|Default|GetHelmet) 0 true)))
          (:then_1
            (Utilities|FlowControl|Delay 1.0)
            (goto _label Reset)))))))

(event Custom|Right%20hand%20punch%20beginplay
  ;[1 1 1] Right Punch
  (Utilities|FlowControl|Sequence
    (:then_0
      (Collision|SetCollisionEnabled (Variables|Default|GetRight%20Hand%20Puncher) "NoCollision"))))

(event EventTick
  (params (DeltaSeconds :type Float%20%28single-precision%29))
  ;[1 1 1] Character Movement
)

(event EventBeginPlay
  ;[1 1 1] Left Punch
  (Utilities|FlowControl|Sequence
    (:then_0
      (Collision|SetCollisionEnabled (Variables|Default|GetLeft%20Hand%20Puncher) "NoCollision"))
    (:then_1
      (CallFunction|RightHandPunchBeginplay))))

(event EventOnLanded
  (params (Hit :type Hit%20Result%20Structure%20%28by%20ref%29))
  ;[1 1 1] Jump mechanics
  (Utilities|FlowControl|Sequence
    (:then_0
      (if (>= 0.6 (Variables|Default|GetJumpHeight))
        (Variables|Default|SetJumpHeight (+ (Variables|Default|GetJumpHeight) 0.2))
        (Utilities|FlowControl|RetriggerableDelay 2.5)
        (Variables|Default|SetJumpHeight 0.4)
        (else
          (Variables|Default|SetJumpHeight 0.4))))))

(event Game|Damage|EventAnyDamage
  (params (Damage :type Float%20%28single-precision%29) (DamageType :type Damage%20Type%20Object%20Reference) (InstigatedBy :type Controller%20Object%20Reference) (DamageCauser :type Actor%20Object%20Reference))
  ;[1 1 1] Damage System
  (if (Variables|Default|GetIs%20injured)
    (Variables|Default|SetHealthBar (- (Variables|Default|GetHealthBar) Damage))
    (Development|PrintString (Utilities|String|ToString(Float) (- (Variables|Default|GetHealthBar) Damage)))
    (CallFunction|DamageImunityTime)))

(event Input|ActionEvents|InputActionToggleRun
  (params (Key :type Key%20Structure :default "None"))
  (:Pressed
    (Variables|/Script/Engine.CharacterMovementComponent|SetMaxWalkSpeed (Variables|Character|GetCharacterMovement) 1e+03))
  (:Released
    (Variables|/Script/Engine.CharacterMovementComponent|SetMaxWalkSpeed (Variables|Character|GetCharacterMovement) 6e+02)))

(event Input|ActionEvents|InputActionJump
  (params (Key :type Key%20Structure :default "None"))
  ;[1 1 1] Jump mechanics
  (:Pressed
    (Variables|Default|SetJumpMaxHoldTime (Variables|Default|GetJumpHeight))
    (Character|Jump)
    (if (>= (Variables|Default|GetJumpHeight) 0.4)
      _))
  (:Released
    (Character|StopJumping)))

(event Input|ActionEvents|InputActionCopy
  (params (Key :type Key%20Structure :default "None"))
  (bind _charactermovement (Variables|Character|GetCharacterMovement))
  (bind _charactermovement_2 (Variables|Character|GetCharacterMovement))
  ;[1 1 1] Copy Ability
  (:Pressed
    (Utilities|FlowControl|DoOnce false :!label _label
      (:Completed
        (bind _returnvalue (Animation|PlayAnimMontage "/Game/Golem/PlayerCharacter/Blueprint/GolumParts/Animations/CopyPowers/Copy.Copy" 1.0 "None"))
        (Utilities|FlowControl|Delay 0.1)
        (Variables|/Script/Engine.CharacterMovementComponent|SetMaxAcceleration _charactermovement_2 4e+04)
        (Variables|/Script/Engine.CharacterMovementComponent|SetMaxWalkSpeed _charactermovement_2 1.5e+04)
        (Timeline|Dash%20Speed PlayFromStart
          (:Update
            (Pawn|Input|AddMovementInput (Math|Vector|GetForwardVector (Variables|Collision|GetCapsuleComponent)) 1.0 false)
            (Utilities|FlowControl|Sequence
              (:then_0
                (Variables|Default|SetIs%20copying true)
                (Utilities|FlowControl|Delay _returnvalue)
                (Variables|Default|SetIs%20copying false))
              (:then_1
                (Variables|Actor|SetbCanBeDamaged false)
                (Utilities|FlowControl|Delay _returnvalue)
                (Variables|Actor|SetbCanBeDamaged true))))
          (:Finished
            (Variables|/Script/Engine.CharacterMovementComponent|SetMaxAcceleration _charactermovement 2048.0)
            (Variables|/Script/Engine.CharacterMovementComponent|SetMaxWalkSpeed _charactermovement 1e+03)
            (Utilities|FlowControl|Delay 0.2)
            (Animation|StopAnimMontage "/Game/Golem/PlayerCharacter/Blueprint/GolumParts/Animations/CopyPowers/Copy.Copy")
            (goto _label Reset)))))))

(event Input|ActionEvents|InputActionRightPunch/Attack
  (params (Key :type Key%20Structure :default "None"))
  (bind _right_hand_puncher (Variables|Default|GetRight%20Hand%20Puncher))
  (:Pressed
    ;[1 1 1] Right Punch
    (if (Variables|Default|GetIsPunching)
      (Utilities|FlowControl|DoOnce false :!label _label
        (:Completed
          (bind _returnvalue (Animation|PlayAnimMontage "/Game/Golem/PlayerCharacter/Blueprint/GolumParts/Animations/Montage/Righthandpunch.Righthandpunch" 1.0 "None"))
          (Utilities|FlowControl|Sequence
            (:then_0
              (Collision|SetCollisionEnabled _right_hand_puncher "QueryAndPhysics")
              (Utilities|FlowControl|Delay _returnvalue)
              (goto _label Reset))
            (:then_1
              (Components|Sphere|SetSphereRadius _right_hand_puncher 32.0 true)
              (Utilities|FlowControl|Delay _returnvalue)
              (Components|Sphere|SetSphereRadius (Variables|Default|GetRight%20Hand%20Puncher) 9.0 true)))))))
  (:Released
    (if (Variables|Default|GetIsPunching)
      (Utilities|FlowControl|Delay 0.5)
      (Collision|SetCollisionEnabled (Variables|Default|GetRight%20Hand%20Puncher) "NoCollision"))))

(event Input|ActionEvents|InputActionLeftPunch/Attack
  (params (Key :type Key%20Structure :default "None"))
  (:Pressed
    ;[1 1 1] Left Punch
    (if (Variables|Default|GetIsPunching)
      (Utilities|FlowControl|DoOnce false :!label _label
        (:Completed
          (bind _returnvalue (Animation|PlayAnimMontage "/Game/Golem/PlayerCharacter/Blueprint/GolumParts/Animations/Montage/PunchAttack.PunchAttack" 1.0 "None"))
          (Utilities|FlowControl|Sequence
            (:then_0
              (Collision|SetCollisionEnabled (Variables|Default|GetLeft%20Hand%20Puncher) "QueryAndPhysics")
              (Utilities|FlowControl|Delay _returnvalue)
              (goto _label Reset))
            (:then_1
              (Components|Sphere|SetSphereRadius (Variables|Default|GetLeft%20Hand%20Puncher) 32.0 true)
              (Utilities|FlowControl|Delay _returnvalue)
              (Components|Sphere|SetSphereRadius (Variables|Default|GetLeft%20Hand%20Puncher) 9.0 true)))))))
  (:Released
    (if (Variables|Default|GetIsPunching)
      (Utilities|FlowControl|Delay 0.5)
      (Collision|SetCollisionEnabled (Variables|Default|GetLeft%20Hand%20Puncher) "NoCollision"))))

(event Input|AxisEvents|InputAxisMoveLeft/Right
  (params (AxisValue :type Float%20%28single-precision%29))
  ;[1 1 1] Character Movement
  (Utilities|FlowControl|Sequence
    (:then_0
      (Pawn|Input|AddMovementInput (Math|Vector|GetRightVector (Math|Rotator|MakeRotator 0.0 0.0 (.Yaw (Math|Rotator|BreakRotator (Pawn|GetControlRotation :!class /Script/Engine.Pawn))))) AxisValue false))))

(event Input|AxisEvents|InputAxisMoveForward/Back
  (params (AxisValue :type Float%20%28single-precision%29))
  ;[1 1 1] Character Movement
  (Utilities|FlowControl|Sequence
    (:then_0
      (Pawn|Input|AddMovementInput (Math|Vector|GetForwardVector (Math|Rotator|MakeRotator 0.0 0.0 (.Yaw (Math|Rotator|BreakRotator (Pawn|GetControlRotation :!class /Script/Engine.Pawn))))) AxisValue false))))

(event Input|AxisEvents|InputAxisRotation
  (params (AxisValue :type Float%20%28single-precision%29))
  ;[1 1 1] Full Rotation
  (Pawn|Input|AddControllerYawInput AxisValue))

(event Input|AxisEvents|InputAxisLookUp/Down
  (params (AxisValue :type Float%20%28single-precision%29))
  ;[1 1 1] Full Rotation
  (Pawn|Input|AddControllerPitchInput AxisValue))

(event Input|KeyboardEvents|LeftCtrl
  (params (Key :type Key%20Structure :default "None"))
  ;[1 1 1] Character Movement
  (:Pressed
    (bind _newtrack_0 (Timeline|Timeline Play)
      (:Update
        (Variables|/Script/Engine.CharacterMovementComponent|SetMaxWalkSpeed (Variables|Character|GetCharacterMovement) (Math|Float|Lerp 6e+02 3e+02 _newtrack_0)))))
  (:Released
    (Timeline|Timeline Reverse)))

(event Input|MouseEvents|RightMouseButton
  (params (Key :type Key%20Structure :default "None"))
  (:Pressed
    (if (not (Variables|Default|GetIsPunching))
      (Variables|Default|Setshooting 1e+01)
      (Variables|Default|Setaiming true)))
  (:Released
    (Variables|Default|Setshooting 0.0)
    (Variables|Default|Setaiming false)))

(event Input|KeyboardEvents|C
  (params (Key :type Key%20Structure :default "None"))
  ;[1 1 1] Copy Ability
  (:Pressed
    (if (Variables|Default|Getactivate%20copy)
      (Variables|Default|Setactivate%20copy false)
      (else
        (Variables|Default|Setactivate%20copy true)))))

(event Input|KeyboardEvents|Tab
  (params (Key :type Key%20Structure :default "None"))
  (:Pressed
    (if (Variables|Default|GetIsPunching)
      (Variables|Default|SetIsPunching false)
      (else
        (Variables|Default|SetIsPunching true)))))

(fn ConstructionScript
  ;[1 1 1] Fuses Parts Together
  (Class|SkinnedMeshComponent|SetMasterPoseComponent (Variables|Default|GetLeft%20Hand) (Variables|Character|GetMesh) false))