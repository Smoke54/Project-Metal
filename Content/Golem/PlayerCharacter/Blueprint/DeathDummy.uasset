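; DeathDummy is a modular golem character, apparently derived from the player, that bursts into pieces on BeginPlay through physical animation on body and head.
; It carries player input for movement, landing-chained higher jumps, a lunging Copy move, camera-offset aiming with ScratchBeam shots, and pause.
; Damage uses a cooldown, and HeadRemover overlaps temporarily clear head meshes.
; Fire-copy and dialogue logic is dormant, and construction-time master-pose linking is disconnected.
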(event OnComponentHit(CapsuleComponent)
  (params (HitComponent :type Primitive%20Component%20Object%20Reference) (OtherActor :type Actor%20Object%20Reference) (OtherComp :type Primitive%20Component%20Object%20Reference) (NormalImpulse :type Vector :default "0, 0, 0") (Hit :type Hit%20Result%20Structure%20%28by%20ref%29))
  ;[1 1 1] Character taking hits
  (Variables|Default|SetIs%20injured true)
  (Utilities|FlowControl|Delay 3.0)
  (Variables|Default|SetIs%20injured false))

(event OnComponentBeginOverlap(HeadSplitter)
  (params (OverlappedComponent :type Primitive%20Component%20Object%20Reference) (OtherActor :type Actor%20Object%20Reference) (OtherComp :type Primitive%20Component%20Object%20Reference) (OtherBodyIndex :type Integer) (bFromSweep :type Boolean) (SweepResult :type Hit%20Result%20Structure%20%28by%20ref%29))
  ;[1 1 1] Detatchable Limbs Feature
  (if (Actor|ActorHasTag OtherActor "HeadRemover")
    (Utilities|FlowControl|DoOnce false :!label _label
      (:Completed
        (Variables|Default|SetRegrowLimb 1)
        (Utilities|FlowControl|Sequence
          (:then_0
            (Utilities|FlowControl|Delay 5.0)
            (Variables|Default|SetRegrowLimb 0)
            (CallFunction|RegrowLeftArm)
            (goto _label Reset))
          (:then_1
            (switch int (Variables|Default|GetRegrowLimb)
              (:0
                (Class|SkinnedMeshComponent|SetSkeletalMesh (Variables|Default|GetHead) "/Game/Golem/PlayerCharacter/Blueprint/GolumParts/Head.Head" true)
                (Class|SkinnedMeshComponent|SetSkeletalMesh (Variables|Default|GetHelmet) "/Game/Golem/PlayerCharacter/Blueprint/GolumParts/Helmet.Helmet" true))
              (:1
                (Class|SkinnedMeshComponent|SetSkeletalMesh (Variables|Default|GetHead) 0 true)
                (Effects|SpawnEmitteratLocation "/Game/StarterContent/Particles/P_Explosion.P_Explosion" (Transformation|GetSocketLocation (Variables|Default|GetHeadSplitter) "Head"))))))))))

(event Custom|Damage%20Imunity%20time
  ;[1 1 1] Character taking hits
  (Variables|Actor|SetbCanBeDamaged false)
  (Utilities|FlowControl|Delay 3.0)
  (Variables|Actor|SetbCanBeDamaged true))

(event Custom|Physical%20Animation%20activation
  ;[1 1 1] Physics (postponed)
)

(event Custom|RegrowLeftArm
  ;[1 1 1] Detatchable Limbs Feature
  (switch int (Variables|Default|GetRegrowLimb)
    (:0
      (Class|SkinnedMeshComponent|SetSkeletalMesh (Variables|Default|GetHead) "/Game/Golem/PlayerCharacter/Blueprint/GolumParts/Head.Head" true)
      (Class|SkinnedMeshComponent|SetSkeletalMesh (Variables|Default|GetHelmet) "/Game/Golem/PlayerCharacter/Blueprint/GolumParts/Helmet.Helmet" true))
    (:1
      (Class|SkinnedMeshComponent|SetSkeletalMesh (Variables|Default|GetHead) 0 true)
      (Effects|SpawnEmitteratLocation "/Game/StarterContent/Particles/P_Explosion.P_Explosion" (Transformation|GetSocketLocation (Variables|Default|GetHeadSplitter) "Head")))))

(event Custom|Transform
  ;[1 1 1] Fire Copy ability(Dormant)
  (if (Variables|Default|GetIs%20copying)
    (Utilities|FlowControl|DoOnce false :!label _label
      (:Completed
        (Utilities|FlowControl|Sequence
          (:then_0
            (if (Variables|Default|GetHas%20Fire)
              (Development|PrintString "fire")
              (Class|SkinnedMeshComponent|SetSkeletalMesh (Variables|Default|GetHead) "/Game/Golem/PlayerCharacter/Blueprint/GolumParts/Transformations/Fire/Fire_Helmet.Fire_Helmet" true)
              (Class|SkinnedMeshComponent|SetSkeletalMesh (Variables|Default|GetHelmet) 0 true)))
          (:then_1
            (Utilities|FlowControl|Delay 1.0)
            (goto _label Reset)))))))

(event Custom|FinnishedWriting_Event_0
  ;[1 1 1] DialogueSystem(Dormant)
  (Utilities|FlowControl|Delay 2.0)
  (if (<= (Variables|Default|Gettextrow) 1)
    (Variables|Default|Settextrow (+ (Variables|Default|Gettextrow) 1))
    (CallFunction|ResetWidget)))

(event Custom|Reset%20Widget
  ;[1 1 1] DialogueSystem(Dormant)
  (Utilities|FlowControl|DoOnce false) ; enters at Reset
)

(event Custom|ignore%20bullet
  (Collision|IgnoreActorwhenMoving (Variables|Collision|GetCapsuleComponent) (.AsScratch%20Beam (Utilities|Casting|CastToScratchBeam (stale EventBeginPlay _output_get))) true :!label _label)
  (Utilities|FlowControl|Delay 0.001)
  (goto _label))

(event Custom|restore%20for%20cutscenes
  ;[1 1 1] Shooting System(Broken
  (if (Variables|Default|Getaiming)
    (Variables|Default|Setaiming false)
    (bind _newtrack_0 (Timeline|Timeline_0 PlayFromStart)
      (:Update
        (Transformation|SetRelativeLocation (Variables|Default|GetCamera) (Math|Vector|Lerp(Vector) "0,20.000000, 0" "0, 0, 0" _newtrack_0) false false)))))

(event Custom|burst%20into%20pieces
  (bind _physicalanimationdata (Utilities|Struct|MakePhysicalAnimationData true 1e+03 1e+02 1e+03 1e+02))
  (bind _physicalanimation (Variables|Default|GetPhysicalAnimation))
  ;[1 1 1] Physics (postponed)
  (Class|PhysicalAnimationComponent|SetSkeletalMeshComponent _physicalanimation (Variables|Character|GetMesh))
  (Class|PhysicalAnimationComponent|ApplyPhysicalAnimationSettingsBelow _physicalanimation (Variables|Default|GetBody%20Name) _physicalanimationdata false)
  (Class|SkeletalMeshComponent|SetAllBodiesBelowSimulatePhysics (Variables|Character|GetMesh) (Variables|Default|GetBody%20Name) true false)
  (Class|PhysicalAnimationComponent|SetSkeletalMeshComponent (Variables|Default|GetPhysicalAnimation) (Variables|Default|GetHead))
  (Class|PhysicalAnimationComponent|ApplyPhysicalAnimationSettingsBelow (Variables|Default|GetPhysicalAnimation) (Variables|Default|GetBody%20Name) _physicalanimationdata false)
  (Class|SkeletalMeshComponent|SetAllBodiesBelowSimulatePhysics (Variables|Default|GetHead) (Variables|Default|GetBody%20Name) true false))

(event EventBeginPlay
  (Utilities|FlowControl|Sequence
    (:then_0
      (Class|PrimitiveComponent|IgnoreComponentwhenMoving (Variables|Default|GetGunHole) (Variables|Collision|GetCapsuleComponent) true)
      (bind _outactors (Actor|GetAllActorsOfClass "/Game/Golem/PlayerCharacter/AttackBlueprints/Weapons/M_GLOW/ScratchBeam.ScratchBeam_C"))
      (bind _output_get (Variables|Default|SetSBREF (Utilities|Array|Get(acopy) _outactors)))
      (Collision|IgnoreActorwhenMoving (Variables|Collision|GetCapsuleComponent) (.AsScratch%20Beam (Utilities|Casting|CastToScratchBeam _output_get)) true :!label _label)
      (Utilities|FlowControl|Delay 0.001)
      (goto _label))
    (:then_1
      (CallFunction|BurstIntoPieces))))

(event EventTick
  (params (DeltaSeconds :type Float%20%28single-precision%29))
  ;[1 1 1] Character Movement
)

(event EventOnLanded
  (params (Hit :type Hit%20Result%20Structure%20%28by%20ref%29))
  ;[1 1 1] Jump mechanics
  (Utilities|FlowControl|Sequence
    (:then_0
      (if (>= 0.6 (Variables|Default|GetJumpHeight))
        (Variables|Default|SetJumpHeight (+ (Variables|Default|GetJumpHeight) 0.2))
        (Utilities|FlowControl|RetriggerableDelay 2.5)
        (Variables|Default|SetJumpHeight 0.4)
        (else
          (Variables|Default|SetJumpHeight 0.4))))))

(event Game|Damage|EventAnyDamage
  (params (Damage :type Float%20%28single-precision%29) (DamageType :type Damage%20Type%20Object%20Reference) (InstigatedBy :type Controller%20Object%20Reference) (DamageCauser :type Actor%20Object%20Reference))
  ;[1 1 1] Damage System
  (Utilities|FlowControl|Sequence
    (:then_0
      (Utilities|FlowControl|DoOnce false :!label _label
        (:Completed
          (Variables|Default|SetHealthBar (- (Variables|Default|GetHealthBar) Damage))
          (bind _returnvalue (Animation|PlayAnimMontage "/Game/Golem/PlayerCharacter/Blueprint/GolumParts/Animations/damage/HurtMontoge.HurtMontoge" 1.0 "None"))
          (Character|LaunchCharacter "0, 0,200.000000" false false)
          (Utilities|FlowControl|Delay _returnvalue)
          (Animation|StopAnimMontage "/Game/Golem/PlayerCharacter/Blueprint/GolumParts/Animations/damage/HurtMontoge.HurtMontoge")
          (Development|PrintString (Utilities|String|ToString(Float) (- (Variables|Default|GetHealthBar) Damage)))
          (if (<= (Variables|Default|GetHealthBar) 0.0)
            (Actor|DestroyActor)
            (else
              (Utilities|FlowControl|Delay 3.0)
              (goto _label Reset))))))))

(event Input|ActionEvents|InputActionShoot
  (params (Key :type Key%20Structure :default "None"))
  (bind _self self)
  ;[1 1 1] default bullet
  (:Pressed
    (if (Variables|Default|Getaiming)
      (Game|SpawnActorfromClass "/Game/Golem/PlayerCharacter/AttackBlueprints/Weapons/M_GLOW/ScratchBeam.ScratchBeam_C" (Transformation|GetWorldTransform (Variables|Default|GetGunHole)) "AlwaysSpawn" _self _self))))

(event Input|ActionEvents|InputActionJump
  (params (Key :type Key%20Structure :default "None"))
  ;[1 1 1] Jump mechanics
  (:Pressed
    (Variables|Default|SetJumpMaxHoldTime (Variables|Default|GetJumpHeight))
    (Character|Jump)
    (if (>= (Variables|Default|GetJumpHeight) 0.4)
      _))
  (:Released
    (Character|StopJumping)))

(event Input|ActionEvents|InputActionCopy
  (params (Key :type Key%20Structure :default "None"))
  ;[1 1 1] Copy Ability
  (:Pressed
    (Utilities|FlowControl|DoOnce false :!label _label
      (:Completed
        (Character|LaunchCharacter "0, 0,400.000000" false false)
        (Utilities|FlowControl|Delay 0.1)
        (Character|LaunchCharacter (* (Math|Vector|GetForwardVector (Transformation|GetActorRotation)) 2.5e+03) false false)
        (Input|DisableInput 0)
        (Animation|PlayAnimMontage "/Game/Golem/PlayerCharacter/Blueprint/GolumParts/Animations/CopyPowers/Copy.Copy" 1.0 "None")
        (Utilities|FlowControl|Delay 0.5)
        (Character|LaunchCharacter (* (Math|Vector|GetForwardVector (Transformation|GetActorRotation)) -2e+03) false false)
        (Animation|StopAnimMontage "/Game/Golem/PlayerCharacter/Blueprint/GolumParts/Animations/CopyPowers/Copy.Copy")
        (Input|EnableInput 0)
        (goto _label Reset)))))

(event Input|ActionEvents|InputActionPause
  (params (Key :type Key%20Structure :default "None"))
  (bind _returnvalue (Game|GetPlayerController 0))
  ;[1 1 1] pause/unpaus
  (:Pressed
    (Utilities|IsValid (Variables|Default|GetPaused)
      (:Is%20Valid
        _)
      (:Is%20Not%20Valid
        (bind _returnvalue_2 (UserInterface|CreateWidget "/Game/HUDS/PauseMenu/Pause.Pause_C"))
        (Variables|Default|SetPaused _returnvalue_2)))
    (if (Game|IsGamePaused)
      (Widget|RemovefromParent (Variables|Default|GetPaused))
      (Game|SetGamePaused false)
      (Variables|/Script/Engine.PlayerController|SetbShowMouseCursor _returnvalue false)
      (Input|SetInputModeGameOnly _returnvalue)
      (else
        (UserInterface|Viewport|AddtoViewport (Variables|Default|GetPaused) 0)
        (Game|SetGamePaused true)
        (Variables|/Script/Engine.PlayerController|SetbShowMouseCursor _returnvalue true)
        (Input|SetInputModeGameandUI _returnvalue (Variables|Default|GetPaused) "LockInFullscreen" false)))))

(event Input|ActionEvents|InputActionTakeAim
  (params (Key :type Key%20Structure :default "None"))
  ;[1 1 1] Shooting System(Broken
  (:Pressed
    (Variables|Default|Setaiming true)
    (bind _newtrack_0 (Timeline|AIMFInger PlayFromStart)
      (:Update
        (Transformation|SetRelativeLocation (Variables|Default|GetCamera) (Math|Vector|Lerp(Vector) "0, 0, 0" "0,20.000000, 0" _newtrack_0) false false))))
  (:Released
    (Variables|Default|Setaiming false)
    (bind _newtrack_0_2 (Timeline|Timeline_0 PlayFromStart)
      (:Update
        (Transformation|SetRelativeLocation (Variables|Default|GetCamera) (Math|Vector|Lerp(Vector) "0,20.000000, 0" "0, 0, 0" _newtrack_0_2) false false)))))

(event Input|AxisEvents|InputAxisMoveLeft/Right
  (params (AxisValue :type Float%20%28single-precision%29))
  ;[1 1 1] Character Movement
  (Utilities|FlowControl|Sequence
    (:then_0
      (Pawn|Input|AddMovementInput (Math|Vector|GetRightVector (Math|Rotator|MakeRotator 0.0 0.0 (.Yaw (Math|Rotator|BreakRotator (Pawn|GetControlRotation :!class /Script/Engine.Pawn))))) AxisValue false))))

(event Input|AxisEvents|InputAxisMoveForward/Back
  (params (AxisValue :type Float%20%28single-precision%29))
  ;[1 1 1] Character Movement
  (Utilities|FlowControl|Sequence
    (:then_0
      (Pawn|Input|AddMovementInput (Math|Vector|GetForwardVector (Math|Rotator|MakeRotator 0.0 0.0 (.Yaw (Math|Rotator|BreakRotator (Pawn|GetControlRotation :!class /Script/Engine.Pawn))))) AxisValue false))))

(event Input|AxisEvents|InputAxisRotation
  (params (AxisValue :type Float%20%28single-precision%29))
  ;[1 1 1] Full Rotation
  (Pawn|Input|AddControllerYawInput AxisValue))

(event Input|AxisEvents|InputAxisLookUp/Down
  (params (AxisValue :type Float%20%28single-precision%29))
  ;[1 1 1] Full Rotation
  (Pawn|Input|AddControllerPitchInput AxisValue))

(event Input|KeyboardEvents|F
  (params (Key :type Key%20Structure :default "None")))

(event Input|KeyboardEvents|F
  (params (Key :type Key%20Structure :default "None"))
  ;[1 1 1] DialogueSystem(Dormant)
)

(fn ConstructionScript
  ;[1 1 1] Fuses Parts Together
)