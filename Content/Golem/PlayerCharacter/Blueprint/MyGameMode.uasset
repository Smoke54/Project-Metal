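; Game mode for the golem game that respawns the player's ShootingGolem after it is destroyed.
; On BeginPlay it binds to the golem's OnDestroyed; on destruction it waits briefly, spawns a replacement at Spawnlocation, possesses it and rebinds through Respawn.
; New players start at the PlayerStart named by the options string minus its first character.
; An unconnected DeathDummy spawn-and-destroy chain never runs.
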(event Custom|On%20Destroyed%20Cust
  (params (DestroyedActor :type Actor%20Object%20Reference))
  (Utilities|FlowControl|Sequence
    (:then_0
      (Utilities|FlowControl|Delay 2.0)
      (bind _returnvalue (Game|SpawnActorfromClass "/Game/Golem/PlayerCharacter/Blueprint/ShootingGolem.ShootingGolem_C" (Variables|Default|GetSpawnlocation) "Undefined" 0 0))
      (Pawn|Possess (Game|GetPlayerController 0) _returnvalue)
      (CallFunction|Respawn))))

(event Custom|Respawn
  (bind _asshooting_golem (Utilities|Casting|CastToShootingGolem (Game|GetPlayerCharacter 0)))
  (Game|BindEventtoOnDestroyed _asshooting_golem (delegate Custom|On%20Destroyed%20Cust)))

(event EventBeginPlay
  (bind _asshooting_golem (Utilities|Casting|CastToShootingGolem (Game|GetPlayerCharacter 0)))
  (Game|BindEventtoOnDestroyed _asshooting_golem (delegate Custom|On%20Destroyed%20Cust)))

(event EventTick
  (params (DeltaSeconds :type Float%20%28single-precision%29)))

(event EventHandleStartingNewPlayer
  (params (NewPlayer :type Player%20Controller%20Object%20Reference))
  (bind _optionsstring (Variables|Default|GetOptionsString))
  (Class|GameModeBase|RestartPlayeratPlayerStart NewPlayer (Class|GameModeBase|FindPlayerStart NewPlayer (Utilities|String|GetSubstring _optionsstring 1 (- (Utilities|String|Len _optionsstring) 1)))))

(fn ConstructionScript)